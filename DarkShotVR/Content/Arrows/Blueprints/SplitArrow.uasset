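; SplitArrow is a projectile arrow actor, apparently for a VR game, that destroys itself five seconds after a hit; no splitting logic appears here.
; Its construction script moves the collision and mesh to a custom channel they ignore, so such objects pass through each other.
; It also sets projectile speeds from ArrowSpeed with a fixed cap and caches the first VR player chaperone found.
; A debug loop repeatedly prints the collision object type.
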(event `self.ReceiveBeginPlay`)

(event `self.ReceiveHit`
  (params (MyComp :type "PrimitiveComponent Object Reference") (Other :type "Actor Object Reference") (OtherComp :type "PrimitiveComponent Object Reference") (bSelfMoved :type Boolean) (HitLocation :type "Vector Structure") (HitNormal :type "Vector Structure") (NormalImpulse :type "Vector Structure") (Hit :type "HitResult Structure (by ref)"))
  (`KismetSystemLibrary.Delay` 5.0)
  (`self.K2_DestroyActor`))

(fn `Init Arrow Speed`
  (bind _projectilemovement (`self.ProjectileMovement`))
  (set `ProjectileMovementComponent.InitialSpeed` (`self.ArrowSpeed`) _projectilemovement)
  (set `ProjectileMovementComponent.MaxSpeed` 5000.0 _projectilemovement))

(fn `Init The Player`
  (bind _outactors (`GameplayStatics.GetAllActorsOfClass` "/Game/Player/MyVR_PlayerChaperone.MyVR_PlayerChaperone_C"))
  (set `self.ThePlayer` (`KismetArrayLibrary.Array_Get` _outactors)))

(fn `Set Collision Channel and Object`
  (bind _arrow_collision (`self.Arrow Collision`))
  (`PrimitiveComponent.SetCollisionResponseToChannel` _arrow_collision "ECC_GameTraceChannel1" "ECR_Ignore")
  (`PrimitiveComponent.SetCollisionResponseToChannel` (`self.Arrow Mesh`) "ECC_GameTraceChannel1" "ECR_Ignore")
  (`PrimitiveComponent.SetCollisionObjectType` _arrow_collision "ECC_GameTraceChannel1")
  (`PrimitiveComponent.SetCollisionObjectType` (`self.Arrow Mesh`) "ECC_GameTraceChannel1")
  (for _ (range 21)
    (`KismetSystemLibrary.PrintString` (`|GetEnumeratorNameAsString` (`PrimitiveComponent.GetCollisionObjectType` _arrow_collision)))))

(fn `UserConstructionScript`
  (`self.Set Collision Channel and Object`)
  (`self.Init Arrow Speed`)
  (`self.Init The Player`))