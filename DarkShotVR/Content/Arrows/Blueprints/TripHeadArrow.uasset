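; TripHeadArrow is a projectile arrow actor that spawns an ExplosiveArrowEffect at its transform when hit, then destroys itself after a zero-length delay.
; The construction script calls Initialize, which caches the first MyVR_PlayerChaperone as Player and sets the projectile's initial and maximum speed.
; Initialize also puts the mesh and box on a custom collision channel they ignore, then repeatedly prints the box's object type as debug output.
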(event `self.ReceiveHit`
  (params (MyComp :type "PrimitiveComponent Object Reference") (Other :type "Actor Object Reference") (OtherComp :type "PrimitiveComponent Object Reference") (bSelfMoved :type Boolean) (HitLocation :type "Vector Structure") (HitNormal :type "Vector Structure") (NormalImpulse :type "Vector Structure") (Hit :type "HitResult Structure (by ref)"))
  (`|SpawnActorFromClass` "/Game/SpecialEffects/ArrowEffects/ExplosiveArrowEffect.ExplosiveArrowEffect_C" (`self.GetTransform`) "Undefined" "OverrideRootScale")
  (`KismetSystemLibrary.Delay` 0.0)
  (`self.K2_DestroyActor`))

(fn `Initialize`
  (bind _projectilemovement (`self.ProjectileMovement`))
  (bind _arrowmesh (`self.ArrowMesh`))
  (bind _outactors (`GameplayStatics.GetAllActorsOfClass` "/Game/Player/MyVR_PlayerChaperone.MyVR_PlayerChaperone_C"))
  (set `self.Player` (`KismetArrayLibrary.Array_Get` _outactors))
  (`PrimitiveComponent.SetCollisionResponseToChannel` _arrowmesh "ECC_GameTraceChannel1" "ECR_Ignore")
  (`PrimitiveComponent.SetCollisionResponseToChannel` (`self.Box`) "ECC_GameTraceChannel1" "ECR_Ignore")
  (`PrimitiveComponent.SetCollisionObjectType` _arrowmesh "ECC_GameTraceChannel1")
  (`PrimitiveComponent.SetCollisionObjectType` (`self.Box`) "ECC_GameTraceChannel1")
  (set `ProjectileMovementComponent.InitialSpeed` (`self.ArrowBaseSpeed`) _projectilemovement)
  (set `ProjectileMovementComponent.MaxSpeed` 5000.0 _projectilemovement)
  (for _ (range 21)
    (`KismetSystemLibrary.PrintString` (`KismetStringLibrary.Conv_ByteToString` (`PrimitiveComponent.GetCollisionObjectType` (`self.Box`))))))

(fn `UserConstructionScript`
  (`self.Initialize`))