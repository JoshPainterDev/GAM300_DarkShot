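; Tripwire arrow projectile for a VR bow, held at the player's left motion controller until fired.
; Construction finds the player chaperone and configures collision and projectile movement; BeginPlay enables input and attaches the arrow to the controller.
; TriggerRelease detaches it, launches it forward at a speed scaled by the player's BowTension, and sets ReadyForSpecial on the player.
; Helper functions measure hand separation, though AmIPullingString is empty.
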(event `self.ReceiveBeginPlay`
  (bind _arrowcollisionbox (`self.ArrowCollisionBox`))
  (bind _l_motioncontrollerscene (`VR_PlayerChaperone.L_MotionControllerScene` (`self.ThePlayer`)))
  (`PrimitiveComponent.SetCollisionResponseToChannel` _arrowcollisionbox "ECC_GameTraceChannel1" "ECR_Ignore")
  (`PrimitiveComponent.SetCollisionResponseToChannel` (`self.C_ArrowMesh`) "ECC_GameTraceChannel1" "ECR_Ignore")
  (`PrimitiveComponent.SetCollisionObjectType` _arrowcollisionbox "ECC_GameTraceChannel1")
  (`PrimitiveComponent.SetCollisionObjectType` (`self.C_ArrowMesh`) "ECC_GameTraceChannel1")
  (`self.EnableInput` null)
  (`SceneComponent.K2_SetWorldLocationAndRotation` (`self.C_ArrowMesh`) (`SceneComponent.K2_GetComponentLocation` _l_motioncontrollerscene) (`SceneComponent.K2_GetComponentRotation` _l_motioncontrollerscene) false false)
  (`self.K2_AttachToComponent` _l_motioncontrollerscene "None" "SnapToTarget" "SnapToTarget" "KeepRelative"))

(event `TriggerRelease`
  (bind _c_projectilemovement (`self.C_ProjectileMovement`))
  (`SceneComponent.K2_DetachFromComponent` (`self.C_ArrowMesh`) "KeepWorld" "KeepWorld" "KeepRelative" true)
  (set `MovementComponent.Velocity` (* (`SceneComponent.GetForwardVector` (`self.C_ArrowMesh`)) (* (+ (`VR_PlayerChaperone._bowTension` (`self.ThePlayer`)) 25.0) 50.0)) _c_projectilemovement)
  (`ActorComponent.SetActive` _c_projectilemovement true false)
  (bind _asmy_vr_player_chaperone (cast `/Game/Blueprints/MyVR_PlayerChaperone` (`self.ThePlayer`)))
  (set `/Game/Blueprints/MyVR_PlayerChaperone.ReadyForSpecial` true _asmy_vr_player_chaperone))

(fn `AmIPullingString`)

(fn `CanAttachToBow`
  (returns (ReturnValue :type Boolean))
  (return (< (`KismetMathLibrary.VSize` (- (`SteamVRFunctionLibrary.GetHandPositionAndOrientation` 0 "Left") (`SteamVRFunctionLibrary.GetHandPositionAndOrientation` 0 "Right"))) 40.0)))

(fn `DistanceBetweenHands`
  (returns (distance :type "Float (double-precision)") (AmIPullingString :type Boolean))
  (bind _returnvalue (`KismetMathLibrary.VSize` (- (`SteamVRFunctionLibrary.GetHandPositionAndOrientation` 0 "Left") (`SteamVRFunctionLibrary.GetHandPositionAndOrientation` 0 "Right"))))
  (return (`KismetMathLibrary.FClamp` _returnvalue 15.0 (`self.MaximumTension`)) (> _returnvalue 40.0)))

(fn `UserConstructionScript`
  (bind _c_projectilemovement (`self.C_ProjectileMovement`))
  (bind _arrowcollisionbox (`self.ArrowCollisionBox`))
  (`PrimitiveComponent.SetCollisionResponseToChannel` _arrowcollisionbox "ECC_GameTraceChannel2" "ECR_Ignore")
  (`PrimitiveComponent.SetCollisionObjectType` _arrowcollisionbox "ECC_GameTraceChannel2")
  (`PrimitiveComponent.SetCollisionObjectType` (`self.C_ArrowMesh`) "ECC_GameTraceChannel2")
  (set `ProjectileMovementComponent.InitialSpeed` 1000.0 _c_projectilemovement)
  (set `ProjectileMovementComponent.MaxSpeed` 5000.0 _c_projectilemovement)
  (bind _outactors (`GameplayStatics.GetAllActorsOfClass` "/Script/DarkShotVR.VR_PlayerChaperone"))
  (set `self.ThePlayer` (`KismetArrayLibrary.Array_Get` _outactors)))