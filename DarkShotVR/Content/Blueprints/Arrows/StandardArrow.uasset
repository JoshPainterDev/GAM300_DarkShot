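; StandardArrow is an arrow projectile Blueprint for what appears to be a VR game.
; Its construction script puts the collision and mesh on a custom trace channel object type that ignores itself, so arrows pass through one another.
; It also sets projectile movement speed from a base arrow speed with a fixed cap, and caches the first VR player chaperone actor found in the world.
; The event graph holds only disabled stub events.
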(fn `Init Projectile Speed`
  (bind _projectilemovement (`self.ProjectileMovement`))
  (set `ProjectileMovementComponent.InitialSpeed` (`self.BaseArrowSpeed`) _projectilemovement)
  (set `ProjectileMovementComponent.MaxSpeed` 5000.0 _projectilemovement))

(fn `Init The Player`
  (bind _outactors (`GameplayStatics.GetAllActorsOfClass` "/Game/MyVR_PlayerChaperone.MyVR_PlayerChaperone_C"))
  (set `self.ThePlayer` (`KismetArrayLibrary.Array_Get` _outactors)))

(fn `Set Collision Channel And Object`
  (bind _arrow_collision (`self.Arrow Collision`))
  (`PrimitiveComponent.SetCollisionResponseToChannel` _arrow_collision "ECC_GameTraceChannel1" "ECR_Ignore")
  (`PrimitiveComponent.SetCollisionResponseToChannel` (`self.ArrowMesh`) "ECC_GameTraceChannel1" "ECR_Ignore")
  (`PrimitiveComponent.SetCollisionObjectType` _arrow_collision "ECC_GameTraceChannel1")
  (`PrimitiveComponent.SetCollisionObjectType` (`self.ArrowMesh`) "ECC_GameTraceChannel1"))

(fn `UserConstructionScript`
  (`self.Set Collision Channel And Object`)
  (`self.Init Projectile Speed`)
  (`self.Init The Player`))