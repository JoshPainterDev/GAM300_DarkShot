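; ExplosiveArrow is a VR arrow projectile Blueprint, though the file contains no explosion logic.
; Separate functions cache the first MyVR_PlayerChaperone as the player, set projectile movement speeds, and put the collision box on a custom channel that ignores itself.
; None of these functions is called within this file; BeginPlay is empty and Tick only prints a debug string.
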(event `self.ReceiveBeginPlay`)

(event `self.ReceiveTick`
  (params (DeltaSeconds :type "Float (single-precision)"))
  (`KismetSystemLibrary.PrintString` "explosive arrow"))

(fn `Init Player`
  (bind _outactors (`GameplayStatics.GetAllActorsOfClass` "/Game/MyVR_PlayerChaperone.MyVR_PlayerChaperone_C"))
  (set `self.ThePlayer` (`KismetArrayLibrary.Array_Get` _outactors)))

(fn `Init Projectile Speed`
  (bind _c_projectilemovement (`self.C_ProjectileMovement`))
  (set `ProjectileMovementComponent.InitialSpeed` 1000.0 _c_projectilemovement)
  (set `ProjectileMovementComponent.MaxSpeed` 5000.0 _c_projectilemovement))

(fn `Set Collision Channel and Object`
  (bind _arrowcollisionbox (`self.ArrowCollisionBox`))
  (`PrimitiveComponent.SetCollisionResponseToChannel` _arrowcollisionbox "ECC_GameTraceChannel1" "ECR_Ignore")
  (`PrimitiveComponent.SetCollisionObjectType` _arrowcollisionbox "ECC_GameTraceChannel1"))

(fn `UserConstructionScript`)