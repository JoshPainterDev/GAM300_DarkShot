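; VR arrow actor for a bow, which starts attached to the player's right motion controller.
; Pressing the right trigger with the hands close together moves the arrow mesh to the left controller as nocked.
; While nocked, Tick sets the player's BowTension from hand distance, and releasing the trigger launches the arrow through ProjectileMovement at tension-scaled speed.
; Attachment and release flags live on the VR_PlayerChaperone found at construction.
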(event `self.ReceiveBeginPlay`
  (bind _theplayer (`self.ThePlayer`))
  (bind _arrowcollisionbox (`self.ArrowCollisionBox`))
  (bind _theplayer_2 (`self.ThePlayer`))
  (bind _r_motioncontrollerscene (`VR_PlayerChaperone.R_MotionControllerScene` _theplayer_2))
  (`PrimitiveComponent.SetCollisionResponseToChannel` _arrowcollisionbox "ECC_GameTraceChannel1" "ECR_Ignore")
  (`PrimitiveComponent.SetCollisionResponseToChannel` (`self.ArrowMesh`) "ECC_GameTraceChannel1" "ECR_Ignore")
  (`PrimitiveComponent.SetCollisionObjectType` _arrowcollisionbox "ECC_GameTraceChannel1")
  (`PrimitiveComponent.SetCollisionObjectType` (`self.ArrowMesh`) "ECC_GameTraceChannel1")
  (`self.EnableInput` null)
  (set `VR_PlayerChaperone._isArrowAttachedToHand` true _theplayer_2)
  (`SceneComponent.K2_SetWorldLocationAndRotation` (`self.ArrowMesh`) (`SceneComponent.K2_GetComponentLocation` _r_motioncontrollerscene) (`SceneComponent.K2_GetComponentRotation` _r_motioncontrollerscene) false false)
  (`self.K2_AttachToComponent` _r_motioncontrollerscene "None" "SnapToTarget" "SnapToTarget" "KeepRelative")
  (`SceneComponent.K2_SetRelativeLocationAndRotation` (`self.ArrowMesh`) (29.0 0.0 0.0) (struct) false false)
  (set `VR_PlayerChaperone._bowTension` 0.0 _theplayer)
  (set `VR_PlayerChaperone._justReleased` false _theplayer))

(event `self.ReceiveTick`
  (params (DeltaSeconds :type "Float (single-precision)"))
  (bind _theplayer (`self.ThePlayer`))
  (if (`VR_PlayerChaperone._isArrowAttachedToBow` _theplayer)
    (bind _distance (`self.DistanceBetweenHands`))
    (set `VR_PlayerChaperone._bowTension` (- _distance 30.0) _theplayer)
    (`KismetSystemLibrary.PrintString` "Pulling Bow")))

(event `Key|MotionController_Right_Trigger`
  (params (Key :type "Key Structure" :default "AnyKey"))
  (bind _theplayer (`self.ThePlayer`))
  (bind _projectilemovement (`self.ProjectileMovement`))
  (bind _theplayer_2 (`self.ThePlayer`))
  (:`Pressed`
    (bind _returnvalue (`self.CanAttachToBow`))
    (if _returnvalue
      (if (`VR_PlayerChaperone._isArrowAttachedToHand` _theplayer_2)
        (for _ (range 21)
          (`KismetSystemLibrary.PrintString` "Hello")
          (`SceneComponent.K2_DetachFromComponent` (`self.ArrowMesh`) "KeepRelative" "KeepRelative" "KeepRelative" true)
          (`SceneComponent.K2_AttachToComponent` (`self.ArrowMesh`) (`VR_PlayerChaperone.L_MotionControllerScene` _theplayer_2) "None" "SnapToTarget" "SnapToTarget" "KeepRelative" true)
          (`SceneComponent.K2_SetRelativeLocationAndRotation` (`self.ArrowMesh`) (0.0 0.0 -9.5) (struct :`Pitch` -90.0 :`Roll` 90.0) false false)
          (set `VR_PlayerChaperone._isArrowAttachedToBow` true _theplayer)
          (set `VR_PlayerChaperone._isArrowAttachedToHand` false _theplayer)))))
  (:`Released`
    (if (`VR_PlayerChaperone._isArrowAttachedToBow` (`self.ThePlayer`))
      (`SceneComponent.K2_DetachFromComponent` (`self.ArrowMesh`) "KeepWorld" "KeepWorld" "KeepRelative" true)
      (set `VR_PlayerChaperone._isArrowAttachedToBow` false (`self.ThePlayer`))
      (set `MovementComponent.Velocity` (* (`SceneComponent.GetForwardVector` (`self.ArrowMesh`)) (* (+ (`VR_PlayerChaperone._bowTension` (`self.ThePlayer`)) 30.0) 10.0)) _projectilemovement)
      (`ActorComponent.SetActive` _projectilemovement true false)
      (set `VR_PlayerChaperone._justReleased` true (`self.ThePlayer`)))))

(fn `AmIPullingString`)

(fn `CanAttachToBow`
  (returns (ReturnValue :type Boolean))
  (return (< (`KismetMathLibrary.VSize` (- (`SteamVRFunctionLibrary.GetHandPositionAndOrientation` 0 "Left") (`SteamVRFunctionLibrary.GetHandPositionAndOrientation` 0 "Right"))) 40.0)))

(fn `DistanceBetweenHands`
  (returns (distance :type "Float (double-precision)") (AmIPullingString :type Boolean))
  (bind _returnvalue (`KismetMathLibrary.VSize` (- (`SteamVRFunctionLibrary.GetHandPositionAndOrientation` 0 "Left") (`SteamVRFunctionLibrary.GetHandPositionAndOrientation` 0 "Right"))))
  (return _returnvalue (> _returnvalue 40.0)))

(fn `UserConstructionScript`
  (bind _projectilemovement (`self.ProjectileMovement`))
  (bind _arrowcollisionbox (`self.ArrowCollisionBox`))
  (`PrimitiveComponent.SetCollisionResponseToChannel` _arrowcollisionbox "ECC_GameTraceChannel2" "ECR_Ignore")
  (`PrimitiveComponent.SetCollisionObjectType` _arrowcollisionbox "ECC_GameTraceChannel2")
  (`PrimitiveComponent.SetCollisionObjectType` (`self.ArrowMesh`) "ECC_GameTraceChannel2")
  (set `ProjectileMovementComponent.InitialSpeed` 1000.0 _projectilemovement)
  (set `ProjectileMovementComponent.MaxSpeed` 5000.0 _projectilemovement)
  (bind _outactors (`GameplayStatics.GetAllActorsOfClass` "/Script/DarkShotVR.VR_PlayerChaperone"))
  (set `self.ThePlayer` (`KismetArrayLibrary.Array_Get` _outactors)))